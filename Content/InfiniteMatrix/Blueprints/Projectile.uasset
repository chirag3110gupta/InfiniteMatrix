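; Player projectile that flies down the world X axis and destroys enemies it hits.
; Each tick it makes a swept move at the player's current forward speed plus a fixed offset, so it outpaces the player.
; Mesh overlap with an Enemy destroys both and increments the player's score, while overlapping a HealthPack or tunnel spawner destroys only the projectile.
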(event `self.ReceiveTick`
  (params (DeltaSeconds :type "Float (single-precision)"))
  (bind _asbp_player (cast `/Game/InfiniteMatrix/Blueprints/BP_Player` (`GameplayStatics.GetPlayerPawn` 0)))
  (`self.K2_AddActorWorldOffset` (`KismetMathLibrary.MakeVector` (* DeltaSeconds (+ (`/Game/InfiniteMatrix/Blueprints/BP_Player.ForwardSpeed` _asbp_player) 1000.0))) true))

(event `self.ProjectileMesh.OnComponentBeginOverlap`
  (params (OverlappedComponent :type "PrimitiveComponent Object Reference") (OtherActor :type "Actor Object Reference") (OtherComp :type "PrimitiveComponent Object Reference") (OtherBodyIndex :type Integer) (bFromSweep :type Boolean) (SweepResult :type "HitResult Structure (by ref)"))
  (bind _asenemy (cast `/Game/InfiniteMatrix/Blueprints/Enemy` OtherActor)
    (:`then`
      (`self.K2_DestroyActor` _asenemy)
      (bind _asbp_player (cast `/Game/InfiniteMatrix/Blueprints/BP_Player` (`GameplayStatics.GetPlayerPawn` 0)))
      (set `/Game/InfiniteMatrix/Blueprints/BP_Player.Player Score` (+ (`/Game/InfiniteMatrix/Blueprints/BP_Player.Player Score` _asbp_player) 1) _asbp_player)
      (`self.K2_DestroyActor`))
    (:`CastFailed`
      (cast `/Game/InfiniteMatrix/Blueprints/HealthPack` OtherActor
        (:`then`
          (`self.K2_DestroyActor`))
        (:`CastFailed`
          (cast `/Game/InfiniteMatrix/Blueprints/BP_TunnelSpawner` OtherActor)
          (`self.K2_DestroyActor`))))))

(fn `UserConstructionScript`)